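; Base floor tile for the runner, which triggers the track's extension and can place coins on itself.
; When BP_CharacterBase overlaps NextFloorSpawner, it calls FAddFloors on BP_GMB and sets a short lifespan so the tile removes itself.
; FAddCoins, not called within this Blueprint, spawns one BP_Coins at a slightly raised random point drawn from the left, middle and right spawn bounds, using NextSpawnLocation's rotation.
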(event OnComponentBeginOverlap(NextFloorSpawner)
  (params (OverlappedComponent :type Primitive%20Component%20Object%20Reference) (OtherActor :type Actor%20Object%20Reference) (OtherComp :type Primitive%20Component%20Object%20Reference) (OtherBodyIndex :type Integer) (bFromSweep :type Boolean) (SweepResult :type Hit%20Result%20Structure%20%28by%20ref%29))
  (bind _asbp_character_base (Utilities|Casting|CastToBP_CharacterBase OtherActor))
  (if (== OtherActor _asbp_character_base)
    (bind _asbp_gmb (Utilities|Casting|CastToBP_GMB (Game|GetGameMode)))
    (Default|FAddFloors _asbp_gmb)
    (Actor|SetLifeSpan 5.0)))

(event EventBeginPlay)

(event Collision|EventActorBeginOverlap
  (params (OtherActor :type Actor%20Object%20Reference)))

(event EventTick
  (params (DeltaSeconds :type Float%20%28single-precision%29)))

(fn ConstructionScript)

(fn FAddCoins
  (bind _returnvalue (Math|Random|RandomIntegerinRange 0 2))
  (bind _spawnleft (Variables|Default|GetSpawnLeft))
  (bind _spawnmiddle (Variables|Default|GetSpawnMiddle))
  (bind _spawnright (Variables|Default|GetSpawnRight))
  (bind (_origin _boxextent) (Collision|GetComponentBounds _spawnright))
  (bind (_origin_2 _boxextent_2) (Collision|GetComponentBounds _spawnleft))
  (bind (_origin_3 _boxextent_3) (Collision|GetComponentBounds _spawnmiddle))
  (bind _returnvalue_2 (Math|Random|RandomPointinBoundingBox _origin _boxextent))
  (bind _returnvalue_3 (Math|Random|RandomPointinBoundingBox _origin_2 _boxextent_2))
  (bind _returnvalue_4 (Math|Random|RandomPointinBoundingBox _origin_3 _boxextent_3))
  (bind _returnvalue_5 (Utilities|Select :Index _returnvalue :Option%200 _returnvalue_3 :Option%201 _returnvalue_4 :Option%202 _returnvalue_2))
  (bind (_x _y _z) (Math|Vector|BreakVector _returnvalue_5))
  (Game|SpawnActorfromClass "/Game/RunnerFolder/Actor/Coins/BP_Coins.BP_Coins_C" (Math|Transform|MakeTransform (Math|Vector|MakeVector _x _y (+ _z 5e+01)) (Transformation|GetWorldRotation (Variables|Default|GetNextSpawnLocation)) "1,1,1") "AdjustIfPossibleButAlwaysSpawn" 0 0))