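; BP_Coins is a runner pickup actor holding five coin components that the player collects to raise a coin count.
; BeginPlay caches the player character and BP_PlayerController.
; Tick spins each remaining coin by a fixed step per frame in alternating directions, not scaled by delta time.
; When the player character overlaps a coin, it increments CurrentCoins on the controller and destroys only that component.
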(event OnComponentBeginOverlap(Coins1)
  (params (OverlappedComponent :type Primitive%20Component%20Object%20Reference) (OtherActor :type Actor%20Object%20Reference) (OtherComp :type Primitive%20Component%20Object%20Reference) (OtherBodyIndex :type Integer) (bFromSweep :type Boolean) (SweepResult :type Hit%20Result%20Structure%20%28by%20ref%29))
  (if (== OtherActor (Variables|Default|GetBP%20Character%20Base%20Ref))
    (Math|Integer|IncrementInt (Variables|/Game/RunnerFolder/PlayerController/BP_PlayerController.BP_PlayerController_C|GetCurrentCoins (Variables|Default|GetBP%20Player%20Controller%20Ref))
      (:%20%20
        (Components|DestroyComponent (Variables|Default|GetCoins1))))))

(event OnComponentBeginOverlap(Coins2)
  (params (OverlappedComponent :type Primitive%20Component%20Object%20Reference) (OtherActor :type Actor%20Object%20Reference) (OtherComp :type Primitive%20Component%20Object%20Reference) (OtherBodyIndex :type Integer) (bFromSweep :type Boolean) (SweepResult :type Hit%20Result%20Structure%20%28by%20ref%29))
  (if (== OtherActor (Variables|Default|GetBP%20Character%20Base%20Ref))
    (Math|Integer|IncrementInt (Variables|/Game/RunnerFolder/PlayerController/BP_PlayerController.BP_PlayerController_C|GetCurrentCoins (Variables|Default|GetBP%20Player%20Controller%20Ref))
      (:%20%20
        (Components|DestroyComponent (Variables|Default|GetCoins2))))))

(event OnComponentBeginOverlap(Coins3)
  (params (OverlappedComponent :type Primitive%20Component%20Object%20Reference) (OtherActor :type Actor%20Object%20Reference) (OtherComp :type Primitive%20Component%20Object%20Reference) (OtherBodyIndex :type Integer) (bFromSweep :type Boolean) (SweepResult :type Hit%20Result%20Structure%20%28by%20ref%29))
  (if (== OtherActor (Variables|Default|GetBP%20Character%20Base%20Ref))
    (Math|Integer|IncrementInt (Variables|/Game/RunnerFolder/PlayerController/BP_PlayerController.BP_PlayerController_C|GetCurrentCoins (Variables|Default|GetBP%20Player%20Controller%20Ref))
      (:%20%20
        (Components|DestroyComponent (Variables|Default|GetCoins3))))))

(event OnComponentBeginOverlap(Coins4)
  (params (OverlappedComponent :type Primitive%20Component%20Object%20Reference) (OtherActor :type Actor%20Object%20Reference) (OtherComp :type Primitive%20Component%20Object%20Reference) (OtherBodyIndex :type Integer) (bFromSweep :type Boolean) (SweepResult :type Hit%20Result%20Structure%20%28by%20ref%29))
  (if (== OtherActor (Variables|Default|GetBP%20Character%20Base%20Ref))
    (Math|Integer|IncrementInt (Variables|/Game/RunnerFolder/PlayerController/BP_PlayerController.BP_PlayerController_C|GetCurrentCoins (Variables|Default|GetBP%20Player%20Controller%20Ref))
      (:%20%20
        (Components|DestroyComponent (Variables|Default|GetCoins4))))))

(event OnComponentBeginOverlap(Coins5)
  (params (OverlappedComponent :type Primitive%20Component%20Object%20Reference) (OtherActor :type Actor%20Object%20Reference) (OtherComp :type Primitive%20Component%20Object%20Reference) (OtherBodyIndex :type Integer) (bFromSweep :type Boolean) (SweepResult :type Hit%20Result%20Structure%20%28by%20ref%29))
  (if (== OtherActor (Variables|Default|GetBP%20Character%20Base%20Ref))
    (Math|Integer|IncrementInt (Variables|/Game/RunnerFolder/PlayerController/BP_PlayerController.BP_PlayerController_C|GetCurrentCoins (Variables|Default|GetBP%20Player%20Controller%20Ref))
      (:%20%20
        (Components|DestroyComponent (Variables|Default|GetCoins5))))))

(event EventBeginPlay
  (bind _asbp_character_base (Utilities|Casting|CastToBP_CharacterBase (Game|GetPlayerCharacter 0)))
  (Variables|Default|SetBP%20Character%20Base%20Ref _asbp_character_base)
  (bind _asbp_player_controller (Utilities|Casting|CastToBP_PlayerController (Game|GetPlayerController 0)))
  (Variables|Default|SetBP%20Player%20Controller%20Ref _asbp_player_controller))

(event Collision|EventActorBeginOverlap
  (params (OtherActor :type Actor%20Object%20Reference)))

(event EventTick
  (params (DeltaSeconds :type Float%20%28single-precision%29))
  (Utilities|FlowControl|Sequence
    (:then_0
      (bind _coins1 (Variables|Default|GetCoins1)
        (:then
          (Transformation|AddLocalRotation _coins1 "0,1.000000, 0" false false))
        (:else)))
    (:then_1
      (bind _coins2 (Variables|Default|GetCoins2)
        (:then
          (Transformation|AddLocalRotation _coins2 "0,-1.000000, 0" false false))
        (:else)))
    (:then_2
      (bind _coins3 (Variables|Default|GetCoins3)
        (:then
          (Transformation|AddLocalRotation _coins3 "0,1.000000, 0" false false))
        (:else)))
    (:then_3
      (bind _coins4 (Variables|Default|GetCoins4)
        (:then
          (Transformation|AddLocalRotation _coins4 "0,-1.000000, 0" false false))
        (:else)))
    (:then_4
      (bind _coins5 (Variables|Default|GetCoins5)
        (:then
          (Transformation|AddLocalRotation _coins5 "0,1.000000, 0" false false))
        (:else)))))

(fn ConstructionScript)