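; Game mode for a runner game that procedurally builds the track by spawning connected floor pieces, six at BeginPlay.
; FAddFloors spawns safe-zone floors until their counter exceeds nine, then straight pieces.
; Once the straight count exceeds a random threshold, rerolled on each check, it spawns a random left or right turn and resets the count.
; Each piece's NextSpawnLocation becomes the transform for the next.
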(event EventBeginPlay
  (for _index (range 0 5)
    (CallFunction|FAddFloors)))

(fn ConstructionScript)

(fn FAddFloors
  (if (> (Variables|Default|GetSafeZoneCounter) 9)
    (if (> (Variables|Default|GetStraightFloorCount) (Math|Random|RandomIntegerinRange 5 (Variables|Default|GetMaxStraightCounter)))
      (bind _returnvalue (Game|SpawnActorfromClass (select (Math|Random|RandomBool) "/Game/RunnerFolder/Actor/BP_TurnRight.BP_TurnRight_C" "/Game/RunnerFolder/Actor/BP_TurnLeft.BP_TurnLeft_C") (Variables|Default|GetSpawn%20Transform) "AlwaysSpawn" 0 0))
      (bind _asbp_floor_base (Utilities|Casting|CastToBP_FloorBase _returnvalue))
      (Variables|Default|SetSpawn%20Transform (Transformation|GetWorldTransform (Variables|/Game/RunnerFolder/Actor/BP_FloorBase.BP_FloorBase_C|GetNextSpawnLocation _asbp_floor_base)))
      (Variables|Default|SetStraightFloorCount 0)
      (else
        (bind _returnvalue_2 (Game|SpawnActorfromClass "/Game/RunnerFolder/Actor/BP_Straight.BP_Straight_C" (Variables|Default|GetSpawn%20Transform) "AlwaysSpawn" 0 0))
        (Variables|Default|SetSpawn%20Transform (Transformation|GetWorldTransform (Variables|/Game/RunnerFolder/Actor/BP_FloorBase.BP_FloorBase_C|GetNextSpawnLocation _returnvalue_2)))
        (Math|Integer|IncrementInt (Variables|Default|GetStraightFloorCount))))
    (else
      (bind _returnvalue_3 (Game|SpawnActorfromClass "/Game/RunnerFolder/Actor/BP_FloorSZ.BP_FloorSZ_C" (Variables|Default|GetSpawn%20Transform) "AlwaysSpawn" 0 0))
      (Variables|Default|SetSpawn%20Transform (Transformation|GetWorldTransform (Variables|/Game/RunnerFolder/Actor/BP_FloorBase.BP_FloorBase_C|GetNextSpawnLocation _returnvalue_3)))
      (Math|Integer|IncrementInt (Variables|Default|GetSafeZoneCounter)))))